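; Game mode that relays task and fail events from its TaskSystem to the SharedHUD widget on BP_HUD.
; Completed tasks show as checked for two seconds, then give way to the current task and next task title, or clear when none remain.
; Progress updates refresh that display immediately, while fails show a timed warning with the fail's title.
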(event `self.TaskSystem.OnTaskUpdate`
  (params (TaskCompleted :type Boolean) (ID :type Integer))
  (bind _tasksystem (`self.TaskSystem`))
  (bind _tasks (`/Game/Blueprints/Components/BP_TaskSystemComponent.Tasks` _tasksystem))
  (bind _currenttaskindex (`/Game/Blueprints/Components/BP_TaskSystemComponent.CurrentTaskIndex` _tasksystem))
  (bind _returnvalue (+ _currenttaskindex 1))
  (bind (_title _score _numsteps _description) (break `/Game/Blueprints/Components/C_TaskData` (`|GetArrayItem` _tasks _currenttaskindex)))
  (bind (_title_2 _score_2 _numsteps_2 _description_2) (break `/Game/Blueprints/Components/C_TaskData` (`|GetArrayItem` _tasks ID)))
  ;[1 0.1967 0.1768] Update Tasks UI
  (bind _asbp_hud (cast `/Game/Blueprints/BP_HUD` (`PlayerController.GetHUD` (`GameplayStatics.GetPlayerController` 0))))
  (if TaskCompleted
    (bind _sharedhud (`/Game/Blueprints/BP_HUD.SharedHUD` _asbp_hud))
    (`/Game/UI/WBP_HUD_Shared.SetCurrentTask` _sharedhud _title_2 _numsteps_2 _numsteps_2 _description_2 true)
    (`KismetSystemLibrary.Delay` 2.0)
    (if (`KismetArrayLibrary.Array_IsValidIndex` _tasks _currenttaskindex)
      (`/Game/UI/WBP_HUD_Shared.SetCurrentTask` _sharedhud _title (`/Game/Blueprints/Components/BP_TaskSystemComponent.CurrentTaskStep` _tasksystem) _numsteps _description false :!label _label)
      (if (`KismetArrayLibrary.Array_IsValidIndex` _tasks _returnvalue)
        (`/Game/UI/WBP_HUD_Shared.SetNextTask` _sharedhud (`.Title_7_5A83EAF748259B5974A34D93B4F0511D` (break `/Game/Blueprints/Components/C_TaskData` (`|GetArrayItem` _tasks _returnvalue))))
        (else
          (`/Game/UI/WBP_HUD_Shared.ClearNextTask` _sharedhud)))
      (else
        (`/Game/UI/WBP_HUD_Shared.ClearCurrentTask` _sharedhud)))
    (else
      (goto _label))))

(event `self.TaskSystem.OnFailUpdate`
  (params (ID :type Integer))
  ;[0.9141 0.2764 1] Update Fails UI
  (bind _asbp_hud (cast `/Game/Blueprints/BP_HUD` (`PlayerController.GetHUD` (`GameplayStatics.GetPlayerController` 0))))
  (`/Game/UI/WBP_HUD_Shared.ShowWarning` (`/Game/Blueprints/BP_HUD.SharedHUD` _asbp_hud) (`.Title_2_283FE8234FCF032A8A6349808A4E32EC` (break `/Game/Blueprints/Components/C_FailData` (`|GetArrayItem` (`/Game/Blueprints/Components/BP_TaskSystemComponent.Fails` (`self.TaskSystem`)) ID))) 3.0))

(fn `UserConstructionScript`)