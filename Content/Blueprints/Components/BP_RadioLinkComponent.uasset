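; Component that handles assembling a radio on its owner from item pickups in a fixed order: back, chip, then front.
; Overlaps on the owner's box collision accept only the next expected "Item"-tagged part, advance the stage, fire OnRadioLinkAttach and destroy the part.
; Tick detects stage changes and sets the Desaturation material parameter on the tagged meshes to distinguish attached from missing parts.
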(event `OnAttachItem`
  (params (OverlappedComponent :type "PrimitiveComponent Object Reference") (OtherActor :type "Actor Object Reference") (OtherComp :type "PrimitiveComponent Object Reference") (OtherBodyIndex :type Integer) (bFromSweep :type Boolean) (SweepResult :type "HitResult Structure (by ref)"))
  (bind _returnvalue (`GameplayStatics.GetObjectClass` OtherActor))
  (if (`Actor.ActorHasTag` OtherActor "Item")
    (switch `int` (`self.Value`)
      (:`0`
        (if (== _returnvalue "/Game/Blueprints/Objects/BP_Radio_Back.BP_Radio_Back_C")
          (`/Engine/EditorBlueprintResources/StandardMacros.IncrementInt` (`self.Value`)
            (:`  `
              (`self.OnRadioLinkAttach` :!label _label)
              (`Actor.K2_DestroyActor` OtherActor)))))
      (:`1`
        (if (== _returnvalue "/Game/Blueprints/Objects/BP_Radio_Chip.BP_Radio_Chip_C")
          (`/Engine/EditorBlueprintResources/StandardMacros.IncrementInt` (`self.Value`)
            (:`  `
              (goto _label)))))
      (:`2`
        (if (== _returnvalue "/Game/Blueprints/Objects/BP_Radio_Front.BP_Radio_Front_C")
          (`/Engine/EditorBlueprintResources/StandardMacros.IncrementInt` (`self.Value`)
            (:`  `
              (goto _label))))))))

(event `self.ReceiveBeginPlay`
  (bind _returnvalue (`self.GetOwner`))
  (set `self.Collision` (`Actor.GetComponentByClass` _returnvalue "/Script/Engine.BoxComponent"))
  (set `self.Front` (`|GetArrayItem` (`Actor.GetComponentsByTag` _returnvalue "/Script/Engine.StaticMeshComponent" "Front")))
  (set `self.Back` (`|GetArrayItem` (`Actor.GetComponentsByTag` _returnvalue "/Script/Engine.StaticMeshComponent" "Back")))
  (set `self.Chip` (`|GetArrayItem` (`Actor.GetComponentsByTag` _returnvalue "/Script/Engine.StaticMeshComponent" "Chip")))
  (add `PrimitiveComponent.OnComponentBeginOverlap` (`self.Collision`) (delegate `OnAttachItem`)))

(event `self.ReceiveTick`
  (params (DeltaSeconds :type "Float (single-precision)"))
  (bind _transparentmeshes (`self.TransparentMeshes`))
  (bind _readymeshes (`self.ReadyMeshes`))
  (bind _transparentmeshes_2 (`self.TransparentMeshes`))
  (bind _readymeshes_2 (`self.ReadyMeshes`))
  (bind _value (`self.Value`))
  (bind _readymeshes_3 (`self.ReadyMeshes`))
  (bind _transparentmeshes_3 (`self.TransparentMeshes`))
  (if (!= _value (`self.OldValue`))
    (`|ExecutionSequence`
      (:`then_0`
        (bind _output_get (set `self.OldValue` _value))
        (switch `int` _output_get
          (:`0`
            (`KismetArrayLibrary.Array_Clear` (`self.ReadyMeshes`))
            (`KismetArrayLibrary.Array_Clear` _transparentmeshes_3)
            (`KismetArrayLibrary.Array_Add` _transparentmeshes_3 (`self.Back`))
            (`KismetArrayLibrary.Array_Add` _transparentmeshes_3 (`self.Chip`))
            (`KismetArrayLibrary.Array_Add` _transparentmeshes_3 (`self.Front`)))
          (:`1`
            (`KismetArrayLibrary.Array_Clear` _readymeshes)
            (`KismetArrayLibrary.Array_Add` _readymeshes (`self.Back`))
            (`KismetArrayLibrary.Array_Clear` _transparentmeshes)
            (`KismetArrayLibrary.Array_Add` _transparentmeshes (`self.Chip`))
            (`KismetArrayLibrary.Array_Add` _transparentmeshes (`self.Front`)))
          (:`2`
            (`KismetArrayLibrary.Array_Clear` _readymeshes_2)
            (`KismetArrayLibrary.Array_Add` _readymeshes_2 (`self.Back`))
            (`KismetArrayLibrary.Array_Add` _readymeshes_2 (`self.Chip`))
            (`KismetArrayLibrary.Array_Clear` _transparentmeshes_2)
            (`KismetArrayLibrary.Array_Add` _transparentmeshes_2 (`self.Front`)))
          (:`3`
            (`KismetArrayLibrary.Array_Clear` _readymeshes_3)
            (`KismetArrayLibrary.Array_Add` _readymeshes_3 (`self.Back`))
            (`KismetArrayLibrary.Array_Add` _readymeshes_3 (`self.Chip`))
            (`KismetArrayLibrary.Array_Add` _readymeshes_3 (`self.Front`))
            (`KismetArrayLibrary.Array_Clear` (`self.TransparentMeshes`)))))
      (:`then_1`
        (for _array_element (`self.ReadyMeshes`)
          (`MeshComponent.SetScalarParameterValueOnMaterials` _array_element "Desaturation" 0.0))
        (for _array_element_2 (`self.TransparentMeshes`)
          (`MeshComponent.SetScalarParameterValueOnMaterials` _array_element_2 "Desaturation" 1.0))))))