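; Actor component that lets its owner receive a radio, consuming the overlapping actor and announcing the pickup.
; On BeginPlay it finds the owner's BoxComponent and binds to its begin-overlap event.
; An overlapping actor whose class exactly matches Filter is destroyed, then the OnRadioReceived dispatcher fires for listeners to react.
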(event `OnRadioReceivedEvent`
  (params (OverlappedComponent :type "PrimitiveComponent Object Reference") (OtherActor :type "Actor Object Reference") (OtherComp :type "PrimitiveComponent Object Reference") (OtherBodyIndex :type Integer) (bFromSweep :type Boolean) (SweepResult :type "HitResult Structure (by ref)"))
  (if (== (`GameplayStatics.GetObjectClass` OtherActor) (`self.Filter`))
    (`Actor.K2_DestroyActor` OtherActor)
    (`self.OnRadioReceived`)))

(event `self.ReceiveBeginPlay`
  (bind _output_get (set `self.Collision` (`Actor.GetComponentByClass` (`self.GetOwner`) "/Script/Engine.BoxComponent")))
  (add `PrimitiveComponent.OnComponentBeginOverlap` _output_get (delegate `OnRadioReceivedEvent`)))