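; BP_TaskSystemComponent is a component that tracks progress through an ordered list of multi-step tasks.
; ReportProgress accepts only the current task's ID, advancing its step or the task and firing update and all-completed events; other IDs count as fail 0.
; ReportFail increments the fail count, deducts that fail's penalty from the clamped score and broadcasts it.
; Task completion leaves the score unchanged, as the score addition is unconnected.
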(fn `ReportFail`
  (params (ID :type Integer))
  (`/Engine/EditorBlueprintResources/StandardMacros.IncrementInt` (`self.FailCount`)
    (:`  `
      (set `self.Score` (`KismetMathLibrary.Clamp` (- (`self.Score`) (`.Score_5_7772D41041C25D16FFF6D28276D8CB54` (break `/Game/Blueprints/Components/C_FailData` (`|GetArrayItem` (`self.Fails`) ID)))) 0 100000))
      (`self.OnFailUpdate` ID))))

(fn `ReportProgress`
  (params (ID :type Integer))
  (bind _currenttaskindex (`self.CurrentTaskIndex`))
  (bind _currenttaskindex_2 (`self.CurrentTaskIndex`))
  (bind (_title _score _numsteps) (break `/Game/Blueprints/Components/C_TaskData` (`|GetArrayItem` (`self.Tasks`) _currenttaskindex)))
  (if (== ID _currenttaskindex)
    (if (and (> _numsteps 1) (!= _numsteps (+ (`self.CurrentTaskStep`) 1)))
      (`/Engine/EditorBlueprintResources/StandardMacros.IncrementInt` (`self.CurrentTaskStep`)
        (:`  `
          (`self.OnTaskUpdate` false _currenttaskindex_2)))
      (else
        (`/Engine/EditorBlueprintResources/StandardMacros.IncrementInt` _currenttaskindex_2
          (:`  `
            (set `self.CurrentTaskStep` 0)
            (set `self.Score` (`self.Score`))
            (`self.OnTaskUpdate` true (- _currenttaskindex_2 1))
            (if (== (`KismetArrayLibrary.Array_Length` (`self.Tasks`)) (`self.CurrentTaskIndex`))
              (`self.OnAllTaskCompleted`))))))
    (else
      (`self.ReportFail` 0))))