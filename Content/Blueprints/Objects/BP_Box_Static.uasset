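; BP_Box_Static is a box actor that is destroyed and counted as a task failure when it touches a box destroyer.
; On BeginPlay it caches the first BP_Box_Static_Spawner found in the level.
; When its Object component overlaps a component tagged BoxDestroyer, it destroys itself, unlocks that spawner's SpawnerComponent and reports a fail to the GameMode's BP_TaskSystemComponent.
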(event `self.ReceiveBeginPlay`
  (bind _outactors (`GameplayStatics.GetAllActorsOfClass` "/Game/Blueprints/Objects/Spawners/BP_Box_Static_Spawner.BP_Box_Static_Spawner_C"))
  (set `self.BoxSpawner` (`|GetArrayItem` _outactors)))

(event `self.Object.OnComponentBeginOverlap`
  (params (OverlappedComponent :type "PrimitiveComponent Object Reference") (OtherActor :type "Actor Object Reference") (OtherComp :type "PrimitiveComponent Object Reference") (OtherBodyIndex :type Integer) (bFromSweep :type Boolean) (SweepResult :type "HitResult Structure (by ref)"))
  (if (`ActorComponent.ComponentHasTag` OtherComp "BoxDestroyer")
    (`self.K2_DestroyActor`)
    (`SpawnerComponent.Unlock` (`self.GetComponentByClass` (`self.BoxSpawner`) "/Script/Factory.SpawnerComponent"))
    (`/Game/Blueprints/Components/BP_TaskSystemComponent.ReportFail` (`self.GetComponentByClass` (`GameplayStatics.GetGameMode`) "/Game/Blueprints/Components/BP_TaskSystemComponent.BP_TaskSystemComponent_C") 1)))

(fn `UserConstructionScript`)