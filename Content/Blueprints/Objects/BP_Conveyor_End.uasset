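; Conveyor end-piece Blueprint that animates its belt surface to match a referenced Conveyor.
; The construction script creates a dynamic instance of M_Conveyor_Belt and applies it to two material slots on the mesh.
; Every tick it sets the material's Speed parameter to the Conveyor's speed, or to zero while that Conveyor is disabled.
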(event `self.ReceiveTick`
  (params (DeltaSeconds :type "Float (single-precision)"))
  (bind _conveyor (`self.Conveyor`))
  (bind _beltmaterial (`self.BeltMaterial`))
  (if (`ConveyorComponent.IsEnabled` _conveyor)
    (`MaterialInstanceDynamic.SetScalarParameterValue` _beltmaterial "Speed" (`ConveyorComponent.Speed` _conveyor))
    (else
      (`MaterialInstanceDynamic.SetScalarParameterValue` _beltmaterial "Speed" 0.0))))

(fn `UserConstructionScript`
  (bind _object (`self.Object`))
  (bind _returnvalue (`KismetMaterialLibrary.CreateDynamicMaterialInstance` "/Game/Objects/Conveyor/M_Conveyor_Belt.M_Conveyor_Belt"))
  (bind _output_get (set `self.BeltMaterial` _returnvalue))
  (`PrimitiveComponent.SetMaterial` _object 1 _output_get)
  (`PrimitiveComponent.SetMaterial` _object 3 _output_get))