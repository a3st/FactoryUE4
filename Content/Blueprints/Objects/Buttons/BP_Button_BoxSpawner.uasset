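; Button Blueprint that requests a new box from a linked spawner object when used.
; Its button action calls Spawn on the SpawnerComponent of BoxSpawnerObject.
; The result drives a timed Russian HUD message saying either that a box is on the way or that the action is unavailable.
; A successful spawn also reports progress to the task system component on the GameMode.
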(event `self.ReceiveBeginPlay`
  (`parent.ReceiveBeginPlay`))

(event `self.Button.OnButtonAction`
  (bind _result (`SpawnerComponent.Spawn` (`self.GetComponentByClass` (`self.BoxSpawnerObject`) "/Script/Factory.SpawnerComponent")))
  (bind _asbp_hud (cast `/Game/Blueprints/BP_HUD` (`PlayerController.GetHUD` (`GameplayStatics.GetPlayerController` 0))))
  (if _result
    (bind _sharedhud (`/Game/Blueprints/BP_HUD.SharedHUD` _asbp_hud))
    (`/Game/UI/WBP_HUD_Shared.ShowInformation` _sharedhud "Новая коробка в пути" 3.0)
    (`/Game/Blueprints/Components/BP_TaskSystemComponent.ReportProgress` (`self.GetComponentByClass` (`GameplayStatics.GetGameMode`) "/Game/Blueprints/Components/BP_TaskSystemComponent.BP_TaskSystemComponent_C") 2)
    (else
      (`/Game/UI/WBP_HUD_Shared.ShowInformation` _sharedhud "В данный момент это действие недоступно" 3.0))))

(fn `UserConstructionScript`
  (`parent.UserConstructionScript`))