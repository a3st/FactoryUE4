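; Conveyor button Blueprint that switches a set of assigned conveyor objects on or off when pressed.
; The button action calls Toggle on each object's ConveyorComponent, then reads the first object's enabled state as the result.
; That state selects a timed Russian on/off message on the shared HUD and which progress ID is reported to the GameMode's task system component.
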(event `self.ReceiveBeginPlay`
  (`parent.ReceiveBeginPlay`))

(event `self.Button.OnButtonAction`
  (bind _conveyorobject (`self.ConveyorObject`))
  (bind _returnvalue (`self.GetComponentByClass` (`GameplayStatics.GetGameMode`) "/Game/Blueprints/Components/BP_TaskSystemComponent.BP_TaskSystemComponent_C"))
  (for _array_element _conveyorobject
    (`ConveyorComponent.Toggle` (`self.GetComponentByClass` _array_element "/Script/Factory.ConveyorComponent")))
  (bind _asbp_hud (cast `/Game/Blueprints/BP_HUD` (`PlayerController.GetHUD` (`GameplayStatics.GetPlayerController` 0))))
  (if (`ConveyorComponent.IsEnabled` (`self.GetComponentByClass` (`|GetArrayItem` _conveyorobject) "/Script/Factory.ConveyorComponent"))
    (bind _sharedhud (`/Game/Blueprints/BP_HUD.SharedHUD` _asbp_hud))
    (`/Game/UI/WBP_HUD_Shared.ShowInformation` _sharedhud "Конвейер вкл." 3.0)
    (`/Game/Blueprints/Components/BP_TaskSystemComponent.ReportProgress` _returnvalue 0)
    (else
      (`/Game/UI/WBP_HUD_Shared.ShowInformation` _sharedhud "Конвейер выкл." 3.0)
      (`/Game/Blueprints/Components/BP_TaskSystemComponent.ReportProgress` _returnvalue 9))))

(fn `UserConstructionScript`
  (`parent.UserConstructionScript`))