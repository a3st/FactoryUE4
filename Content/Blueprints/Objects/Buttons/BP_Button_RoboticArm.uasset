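; Button Blueprint that switches a referenced robotic arm on or off when pressed.
; The press calls Toggle on the arm's RoboticArmComponent, then shows a timed Russian HUD message for on, off or action unavailable.
; A successful toggle also reports progress to the game mode's task system, with a different ID for the enabled and disabled states.
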(event `self.ReceiveBeginPlay`
  (`parent.ReceiveBeginPlay`))

(event `self.Button.OnButtonAction`
  (bind _returnvalue (`self.GetComponentByClass` (`self.RoboticArmObject`) "/Script/Factory.RoboticArmComponent"))
  (bind _returnvalue_2 (`self.GetComponentByClass` (`GameplayStatics.GetGameMode`) "/Game/Blueprints/Components/BP_TaskSystemComponent.BP_TaskSystemComponent_C"))
  (bind _returnvalue_3 (`RoboticArmComponent.Toggle` _returnvalue))
  (bind _asbp_hud (cast `/Game/Blueprints/BP_HUD` (`PlayerController.GetHUD` (`GameplayStatics.GetPlayerController` 0))))
  (if _returnvalue_3
    (if (`RoboticArmComponent.IsEnabled` _returnvalue)
      (bind _sharedhud (`/Game/Blueprints/BP_HUD.SharedHUD` _asbp_hud))
      (`/Game/UI/WBP_HUD_Shared.ShowInformation` _sharedhud "Механическая рука вкл." 3.0)
      (`/Game/Blueprints/Components/BP_TaskSystemComponent.ReportProgress` _returnvalue_2 1)
      (else
        (`/Game/UI/WBP_HUD_Shared.ShowInformation` _sharedhud "Механическая рука выкл." 3.0)
        (`/Game/Blueprints/Components/BP_TaskSystemComponent.ReportProgress` _returnvalue_2 8)))
    (else
      (`/Game/UI/WBP_HUD_Shared.ShowInformation` _sharedhud "В данный момент это действие недоступно" 3.0))))

(fn `UserConstructionScript`
  (`parent.UserConstructionScript`))