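; First-person player Blueprint that handles look input and drives HUD feedback for whatever the camera points at.
; Interact press and release are forwarded to Player, whose InteractDistance also sets the length of a camera line trace run every Tick.
; Hits tagged "Button" enable interactive mode; other results clear it and hide the target.
; Hit actors with a BP_TargetUIComponent then show name, danger and safe distance while this pawn is possessed.
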(event `InputAxis|LookLeft`
  (params (AxisValue :type "Float (single-precision)"))
  (`self.AddControllerYawInput` AxisValue))

(event `InputAxis|LookUp`
  (params (AxisValue :type "Float (single-precision)"))
  (`self.AddControllerPitchInput` AxisValue))

(event `InputAction|Interact`
  (params (Key :type "Key Structure"))
  (bind _player (`self.Player`))
  (:`Pressed`
    (`PlayerComponent.PressInteract` _player))
  (:`Released`
    (`PlayerComponent.ReleaseInteract` _player)))

(event `self.ReceiveTick`
  (params (DeltaSeconds :type "Float (single-precision)"))
  (bind _returnvalue (`GameplayStatics.GetPlayerController` 0))
  (bind _camera (`self.Camera`))
  (bind _returnvalue_2 (`SceneComponent.K2_GetComponentLocation` _camera))
  (bind _returnvalue_3 (`PlayerController.GetHUD` (`GameplayStatics.GetPlayerController` 0)))
  (bind (_outhit _returnvalue_4) (`KismetSystemLibrary.LineTraceSingle` _returnvalue_2 (+ _returnvalue_2 (* (`KismetMathLibrary.GetForwardVector` (`SceneComponent.K2_GetComponentRotation` _camera)) (`PlayerComponent.InteractDistance` (`self.Player`)))) "TraceTypeQuery2"))
  (if _returnvalue_4
    (`|ExecutionSequence`
      (:`then_0`
        (bind (_bblockinghit _binitialoverlap _time _distance _location _impactpoint _normal _impactnormal _physmat _hitactor) (`GameplayStatics.BreakHitResult` _outhit))
        ;[1 0.2546 0.9624] Interactive Mode
        (if (`self.ActorHasTag` _hitactor "Button")
          (bind _asbp_hud (cast `/Game/Blueprints/BP_HUD` _returnvalue_3))
          (`/Game/UI/WBP_HUD_FP.SetInteractiveMode` (`/Game/Blueprints/BP_HUD.FPHUD` _asbp_hud) true)
          (else
            (bind _asbp_hud_2 (cast `/Game/Blueprints/BP_HUD` _returnvalue_3 :!label _label))
            (`/Game/UI/WBP_HUD_FP.SetInteractiveMode` (`/Game/Blueprints/BP_HUD.FPHUD` _asbp_hud_2) false)
            (`/Game/UI/WBP_HUD_Shared.HideTarget` (`/Game/Blueprints/BP_HUD.SharedHUD` _asbp_hud_2)))))
      (:`then_1`
        (bind _returnvalue_5 (`self.GetComponentByClass` _hitactor "/Game/UI/BP_TargetUIComponent.BP_TargetUIComponent_C"))
        ;[0.3739 0.5234 1] Target
        (`/Engine/EditorBlueprintResources/StandardMacros.IsValid` _returnvalue_5
          (:`Is Valid`
            (if (== (`Controller.K2_GetPawn` _returnvalue) self)
              (bind _asbp_hud_3 (cast `/Game/Blueprints/BP_HUD` (`PlayerController.GetHUD` _returnvalue)))
              (`/Game/UI/WBP_HUD_Shared.ShowTarget` (`/Game/Blueprints/BP_HUD.SharedHUD` _asbp_hud_3) (`/Game/UI/BP_TargetUIComponent.Name` _returnvalue_5) (`/Game/UI/BP_TargetUIComponent.IsDanger` _returnvalue_5) (`/Game/UI/BP_TargetUIComponent.SafeDistance` _returnvalue_5)))))))
    (else
      (goto _label))))

(fn `UserConstructionScript`)